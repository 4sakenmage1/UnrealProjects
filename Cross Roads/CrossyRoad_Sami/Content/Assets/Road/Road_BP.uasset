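; Road tile for a Crossy Road-style game that spawns YellowCar traffic crossing along the Y axis.
; BeginPlay randomly picks the left or right spawn side, fixing car direction and rotation.
; Tick spawns cars by delta-scaled chance after MinimumSpawnTime, though the post-spawn reset writes a separate NextMinimumSpawnTime variable that check never reads.
; A CrossRoadAss actor overlapping the trigger calls its SpawnNextTile.
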(event OnComponentBeginOverlap(Trigger)
  (params (OverlappedComponent :type Primitive%20Component%20Object%20Reference) (OtherActor :type Actor%20Object%20Reference) (OtherComp :type Primitive%20Component%20Object%20Reference) (OtherBodyIndex :type Integer) (bFromSweep :type Boolean) (SweepResult :type Hit%20Result%20Structure%20%28by%20ref%29))
  (bind _ascross_road_ass (Utilities|Casting|CastToCrossRoadAss OtherActor))
  (Default|SpawnNextTile _ascross_road_ass))

(event EventBeginPlay
  (CallFunction|InitializeSpawnPoint))

(event EventTick
  (params (DeltaSeconds :type Float%20%28single-precision%29))
  (CallFunction|ChancetoSpawn DeltaSeconds))

(fn ConstructionScript)

(fn ChancetoSpawn
  (params (DeltaSeconds :type Float%20%28single-precision%29))
  (bind _spawncar (CallFunction|CheckSpawnDelay))
  (if _spawncar
    (if (> (* DeltaSeconds (Variables|Default|GetSpawnChance)) (Math|Random|RandomFloat))
      (CallFunction|SpawnCar))))

(fn CheckSpawnDelay
  (return (> (Utilities|Time|GetGameTimeinSeconds) (Variables|Default|GetMinimumSpawnTime))))

(fn SpawnCar
  (bind _returnvalue (Game|SpawnActorfromClass "/Game/BluePrints/YellowCar.YellowCar_C" (Math|Transform|MakeTransform (Variables|Default|GetSpawnPoint) "0, 0, 0" "1,1,1") "Undefined" 0 0))
  (Variables|/Game/BluePrints/YellowCar.YellowCar_C|SetSpeedDirection _returnvalue (Math|Vector|MakeVector 0.0 (Variables|Default|GetCarDirection_Y) 0.0))
  (Default|SetRotation _returnvalue (Variables|Default|GetVehicleRotation))
  (CallFunction|ResetSpawnDelay))

(fn ResetSpawnDelay
  (Variables|Default|SetNextMinimumSpawnTime (+ (Variables|Default|GetInit_Delay) (Utilities|Time|GetGameTimeinSeconds))))

(fn InitializeSpawnPoint
  (bind _spawnleft (Variables|Default|GetSpawnLeft))
  (bind _spawnright (Variables|Default|GetSpawnRight))
  (bind _returnvalue (Transformation|GetWorldLocation _spawnleft))
  (bind _returnvalue_2 (Transformation|GetWorldLocation _spawnright))
  (if (Math|Random|RandomBool)
    (Variables|Default|SetSpawnPoint (Math|Vector|MakeVector (.x _returnvalue) (.y _returnvalue) 2e+01))
    (Variables|Default|SetCarDirection_Y 1.0)
    (Variables|Default|SetVehicleRotation "0,90.000000, 0")
    (else
      (Variables|Default|SetSpawnPoint (Math|Vector|MakeVector (+ 1e+02 (.x _returnvalue_2)) (.y _returnvalue_2) 2e+01))
      (Variables|Default|SetCarDirection_Y -1.0)
      (Variables|Default|SetVehicleRotation "0,270.000000, 0"))))