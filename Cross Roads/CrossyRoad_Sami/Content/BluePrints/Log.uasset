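; Moving log actor that travels along SpeedDirection at Speed and carries the player with it while in contact.
; Every tick UseSpeed offsets the log, and also the player pawn when IsDragging is set; CheckDragging refreshes that flag on a 0.05-second throttle from overlaps with McCarthy.
; A Delay on Tick destroys the log after ten seconds.
; SetRotation sets the log's world rotation; older respawn logic is left disconnected.
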(event EventBeginPlay)

(event Collision|EventActorBeginOverlap
  (params (OtherActor :type Actor%20Object%20Reference)))

(event EventTick
  (params (DeltaSeconds :type Float%20%28single-precision%29))
  (CallFunction|UseSpeed DeltaSeconds)
  (CallFunction|CheckDragging)
  (Utilities|FlowControl|Delay 1e+01)
  (Actor|DestroyActor))

(fn ConstructionScript)

(fn SetRotation
  (params (Rotation :type Rotator))
  (Transformation|SetWorldRotation (Variables|Default|GetLog) Rotation false false))

(fn UseSpeed
  (params (DeltaSeconds :type Float%20%28single-precision%29))
  (bind _speeddirection (Variables|Default|GetSpeedDirection))
  (bind _speed (Variables|Default|GetSpeed))
  (bind _returnvalue (* _speeddirection DeltaSeconds))
  (bind _returnvalue_2 (* _returnvalue _speed))
  (Transformation|AddActorWorldOffset _returnvalue_2)
  (if (Variables|Default|GetisDragging)
    (Transformation|AddActorWorldOffset (Game|Player|GetPlayerPawn 0) _returnvalue_2)))

(fn CheckDragging
  (bind _returnvalue (Utilities|Time|GetGameTimeinSeconds))
  (if (> _returnvalue (Variables|Default|GetNextDraggingPlayer))
    (Variables|Default|SetNextDraggingPlayer (+ _returnvalue 0.05))
    (if (> (Utilities|Array|Length (Collision|GetOverlappingActors "/Game/BluePrints/McCarthy.McCarthy_C" :!class /Script/Engine.Actor)) 0)
      (Variables|Default|SetisDragging true)
      (else
        (Variables|Default|SetisDragging false)))))