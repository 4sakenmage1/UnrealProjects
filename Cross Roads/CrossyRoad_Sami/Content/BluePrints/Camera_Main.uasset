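; Main game camera actor that follows the first player forward along world X and can auto-scroll.
; Construction clears the Scroll flag and places the root at PlayerVector; BeginPlay aims the camera at the player once.
; Each tick pushes X up to the player's plus MinPlayerVector, never backward, then adds ScrollSpeed movement if Scroll is set.
; GetView makes this actor the player controller's view target.
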(event EventBeginPlay
  (CallFunction|FacePlayer))

(event Collision|EventActorBeginOverlap
  (params (OtherActor :type Actor%20Object%20Reference)))

(event EventTick
  (params (DeltaSeconds :type Float%20%28single-precision%29))
  (Utilities|FlowControl|Sequence
    (:then_0
      (CallFunction|PlayerCam))
    (:then_1
      (CallFunction|CheckScroll DeltaSeconds))))

(fn ConstructionScript
  (Utilities|FlowControl|Sequence
    (:then_0
      (CallFunction|HaltScroll))
    (:then_1
      (Transformation|SetWorldLocation (Variables|Default|GetDefaultSceneRoot) (Variables|Default|GetPlayerVector) false false))))

(fn HaltScroll
  (Variables|Default|SetScroll? false))

(fn CheckScroll
  (params (DeltaSeconds :type Float%20%28single-precision%29))
  (if (Variables|Default|GetScroll?)
    (CallFunction|Scroll DeltaSeconds)))

(fn Scroll
  (params (DeltaSeconds :type Float%20%28single-precision%29))
  (Transformation|SetWorldLocation (Variables|Default|GetDefaultSceneRoot) (+ (* (Variables|Default|GetScrollSpeed_) DeltaSeconds) (Transformation|GetWorldLocation (Variables|Default|GetDefaultSceneRoot))) false false))

(fn PlayerCam
  (bind _returnvalue (Game|Player|GetPlayerPawn 0))
  (bind _defaultsceneroot (Variables|Default|GetDefaultSceneRoot))
  (bind _minplayervector (Variables|Default|GetMinPlayerVector))
  (bind _returnvalue_2 (Transformation|GetWorldLocation _defaultsceneroot))
  (bind _rootcomponent (Variables|/Script/Engine.Actor|GetRootComponent _returnvalue))
  (bind _returnvalue_3 (Transformation|GetWorldLocation _rootcomponent))
  (bind _returnvalue_4 (+ (.x _returnvalue_3) _minplayervector))
  (if (Utilities|IsValid _returnvalue)
    (if (< (.x _returnvalue_2) _returnvalue_4)
      (Transformation|SetWorldLocation (Variables|Default|GetDefaultSceneRoot) (Math|Vector|MakeVector _returnvalue_4 (.y _returnvalue_2) (.z _returnvalue_2)) false false))))

(fn FacePlayer
  (bind _returnvalue (Game|Player|GetPlayerPawn 0))
  (if (Utilities|IsValid _returnvalue)
    (Utilities|FlowControl|Sequence
      (:then_0
        (CallFunction|PlayerCam))
      (:then_1
        (Transformation|SetWorldRotation (Variables|Default|GetCamera) (Math|Conversions|RotationFromXVector (Math|Vector|GetUnitDirection(Vector) (Transformation|GetWorldLocation (Variables|Default|GetCamera)) (Transformation|GetWorldLocation (Variables|/Script/Engine.Actor|GetRootComponent _returnvalue)))) false false)))))

(fn GetView
  (Game|Player|SetViewTargetwithBlend (Game|GetPlayerController 0) self 0.0 "VTBlend_Linear" 0.0 false)
  (return false))