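; Player character for a Crossy Road-style hopper, moved on a grid by releasing directional inputs.
; Each hop turns the mesh, jumps and teleports about 100 units, snapped to 50-unit steps; the first also starts the round and menu animation.
; Hitting a car, train or water sets IsDead, making Tick flatten the capsule and pin the camera; WallCollide restores the previous location.
; Interpolated-jump and Reset helpers exist but are not called here.
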(event Collision|EventHit
  (params (MyComp :type Primitive%20Component%20Object%20Reference) (Other :type Actor%20Object%20Reference) (OtherComp :type Primitive%20Component%20Object%20Reference) (bSelfMoved :type Boolean) (HitLocation :type Vector :default "0, 0, 0") (HitNormal :type Vector :default "0, 0, 0") (NormalImpulse :type Vector :default "0, 0, 0") (Hit :type Hit%20Result%20Structure%20%28by%20ref%29))
  (if (not (Variables|Default|GetisDead))
    (Utilities|Casting|CastToYellowCar Other
      (:then
        _)
      (:CastFailed
        (Utilities|Casting|CastToTrain Other
          (:then
            _)
          (:CastFailed
            (bind _aswater_bp (Utilities|Casting|CastToWater_BP Other))
            (Class|PrimitiveComponent|BoxOverlapComponent :self (Variables|/Game/Assets/Water/Water_BP.Water_BP_C|GetDrowing _aswater_bp))))))
    (Variables|Default|SetisDead true)))

(event EventTick
  (params (DeltaSeconds :type Float%20%28single-precision%29))
  (bind _location (Variables|Default|GetLocation))
  (if (Variables|Default|GetisDead)
    (Transformation|SetWorldTransform (Variables|Collision|GetCapsuleComponent) (Math|Transform|MakeTransform (Math|Vector|MakeVector (.x _location) (.y _location) 1e+01) "0, 0, 0" "1.000000,1.000000,0.100000") false false)
    (Transformation|SetWorldTransform (Variables|Default|GetCamera) (Math|Transform|MakeTransform (Variables|Default|GetGetCameraLocation) (Variables|Default|GetGetCameraRotation) "1,1,1") false false)
    (elif (Variables|Default|GetWallCollide)
      (Transformation|SetWorldLocation (Variables|Collision|GetCapsuleComponent) (Variables|Default|GetPreviousLocation) false false)
      (Variables|Default|SetWallCollide false))))

(event EventBeginPlay
  (CallFunction|InitializePlayer)
  (bind _returnvalue (UserInterface|CreateWidget "/Game/BluePrints/Menu.Menu_C"))
  (bind _output_get (Variables|Default|SetUI _returnvalue))
  (UserInterface|Viewport|AddtoViewport _output_get 0)
  (Default|Animation (Variables|Default|GetUI)))

(event Collision|EventActorBeginOverlap
  (params (OtherActor :type Actor%20Object%20Reference)))

(event Input|ActionEvents|InputActionMoveForward
  (params (Key :type Key%20Structure))
  (bind _returnvalue (Transformation|GetActorLocation))
  (bind _camera (Variables|Default|GetCamera))
  (:Released
    (if (Variables|Default|GetRoundStart)
      _
      (else
        (Variables|Default|SetRoundStart true)
        (Default|Animation2 (Variables|Default|GetUI))))
    (if (not (Variables|Default|GetIsJumping))
      (Transformation|SetRelativeRotation (Variables|Character|GetMesh) "0, 0, 0" false false)
      (Variables|Default|SetIsJumping true)
      (Character|Jump)
      (Variables|Default|SetPreviousLocation (Math|Vector|MakeVector (.x _returnvalue) (.y _returnvalue) (.z _returnvalue)))
      (Utilities|FlowControl|Sequence
        (:then_0
          (bind _rounded (CallFunction|RoundtotheNearest50 (+ 1e+02 (.x _returnvalue)))))
        (:then_1
          (Transformation|SetActorRelativeLocation (Math|Vector|MakeVector _rounded (.y _returnvalue) (.z _returnvalue)))
          (Utilities|FlowControl|Delay 0.1)
          (Variables|Default|SetIsJumping false)
          (Variables|Default|SetLocation (Transformation|GetActorLocation))
          (Variables|Default|SetGetCameraLocation (Transformation|GetWorldLocation _camera))
          (Variables|Default|SetGetCameraRotation (Transformation|GetWorldRotation _camera)))))))

(event Input|ActionEvents|InputActionMoveBack
  (params (Key :type Key%20Structure))
  (bind _returnvalue (Transformation|GetActorLocation))
  (bind _camera (Variables|Default|GetCamera))
  (:Released
    (if (Variables|Default|GetRoundStart)
      _
      (else
        (Variables|Default|SetRoundStart true)
        (Default|Animation2 (Variables|Default|GetUI))))
    (if (not (Variables|Default|GetIsJumping))
      (Transformation|SetRelativeRotation (Variables|Character|GetMesh) "0,180.000000, 0" false false)
      (Variables|Default|SetIsJumping true)
      (Character|Jump)
      (Variables|Default|SetPreviousLocation (Math|Vector|MakeVector (.x _returnvalue) (.y _returnvalue) (.z _returnvalue)))
      (Utilities|FlowControl|Sequence
        (:then_0
          (bind _rounded (CallFunction|RoundtotheNearest50 (+ -1e+02 (.x _returnvalue)))))
        (:then_1
          (Transformation|SetActorRelativeLocation (Math|Vector|MakeVector _rounded (.y _returnvalue) (.z _returnvalue)))
          (Utilities|FlowControl|Delay 0.1)
          (Variables|Default|SetIsJumping false)
          (Variables|Default|SetLocation (Transformation|GetActorLocation))
          (Variables|Default|SetGetCameraLocation (Transformation|GetWorldLocation _camera))
          (Variables|Default|SetGetCameraRotation (Transformation|GetWorldRotation _camera)))))))

(event Input|ActionEvents|InputActionMoveRight
  (params (Key :type Key%20Structure))
  (bind _returnvalue (Transformation|GetActorLocation))
  (bind _camera (Variables|Default|GetCamera))
  (:Released
    (if (Variables|Default|GetRoundStart)
      _
      (else
        (Variables|Default|SetRoundStart true)
        (Default|Animation2 (Variables|Default|GetUI))))
    (if (not (Variables|Default|GetIsJumping))
      (Transformation|SetRelativeRotation (Variables|Character|GetMesh) "0,-270.000000, 0" false false)
      (Variables|Default|SetIsJumping true)
      (Character|Jump)
      (if (Variables|Default|GetWallCollide)
        (Utilities|FlowControl|Delay 0.1)
        (Variables|Default|SetIsJumping false)
        (else
          (Variables|Default|SetPreviousLocation (Math|Vector|MakeVector (.x _returnvalue) (.y _returnvalue) (.z _returnvalue)))
          (bind _rounded (CallFunction|RoundtotheNearest50 (+ 1e+02 (.y _returnvalue))))
          (Transformation|SetWorldLocation (Variables|Collision|GetCapsuleComponent) (Math|Vector|MakeVector (.x _returnvalue) _rounded (.z _returnvalue)) false false)
          (Utilities|FlowControl|Delay 0.1)
          (Variables|Default|SetIsJumping false)
          (Variables|Default|SetLocation (Transformation|GetActorLocation))
          (Variables|Default|SetGetCameraLocation (Transformation|GetWorldLocation _camera))
          (Variables|Default|SetGetCameraRotation (Transformation|GetWorldRotation _camera)))))))

(event Input|ActionEvents|InputActionMoveLeft
  (params (Key :type Key%20Structure))
  (bind _returnvalue (Transformation|GetActorLocation))
  (bind _camera (Variables|Default|GetCamera))
  (:Released
    (if (Variables|Default|GetRoundStart)
      _
      (else
        (Variables|Default|SetRoundStart true)
        (Default|Animation2 (Variables|Default|GetUI))))
    (if (not (Variables|Default|GetIsJumping))
      (Transformation|SetRelativeRotation (Variables|Character|GetMesh) "0,270.000000, 0" false false)
      (Variables|Default|SetIsJumping true)
      (Character|Jump)
      (if (Variables|Default|GetWallCollide)
        (Utilities|FlowControl|Delay 0.1)
        (Variables|Default|SetIsJumping false)
        (else
          (Variables|Default|SetPreviousLocation (Math|Vector|MakeVector (.x _returnvalue) (.y _returnvalue) (.z _returnvalue)))
          (Utilities|FlowControl|Sequence
            (:then_0
              (bind _rounded (CallFunction|RoundtotheNearest50 (+ (.y _returnvalue) -1e+02))))
            (:then_1
              (Transformation|SetActorRelativeLocation (Math|Vector|MakeVector (.x _returnvalue) _rounded (.z _returnvalue)))
              (Utilities|FlowControl|Delay 0.1)
              (Variables|Default|SetIsJumping false)
              (Variables|Default|SetLocation (Transformation|GetActorLocation))
              (Variables|Default|SetGetCameraLocation (Transformation|GetWorldLocation _camera))
              (Variables|Default|SetGetCameraRotation (Transformation|GetWorldRotation _camera)))))))))

(fn ConstructionScript)

(fn Movement
  (params (Delta%20Seconds :type Float%20%28single-precision%29)))

(fn PerformJump
  (params (DeltaSeconds :type Float%20%28single-precision%29))
  (if (Variables|Default|GetIsJumping)
    (bind _jumplocation (CallFunction|JumpAction DeltaSeconds))
    (bind _remainingdistance (CallFunction|JumpCheckDistance))
    (if (> (Math|Vector|VectorLength _remainingdistance) (Math|Vector|VectorLength _jumplocation))
      (Transformation|AddActorLocalOffset _jumplocation true false)
      (else
        (Transformation|SetActorLocation (Variables|Default|GetLocation) false false)
        (Variables|Default|SetIsJumping false)))))

(fn JumpAction
  (params (Delta%20Seconds :type Float%20%28single-precision%29))
  (if (Variables|Default|GetIsJumping)
    (return (* (* (Math|Vector|Normalize (- (Variables|Default|GetLocation) (Transformation|GetActorLocation))) Delta%20Seconds) (Variables|Default|GetMax_Speed)))))

(fn JumpCheckDistance
  (return (- (Variables|Default|GetLocation) (Transformation|GetActorLocation))))

(fn ReadyForward
  (bind _canjump (CallFunction|CheckJump))
  (if _canjump
    (Transformation|SetActorRotation "0, 0, 0")))

(fn CheckJump
  (return (Math|Boolean|ANDBoolean (Variables|/Game/BluePrints/CrossRoadAss.CrossRoadAss_C|GetIsPlaying (Variables|Default|GetGame)) (not (Variables|Default|GetIsJumping)) (not (Variables|Default|GetisDead)))))

(fn Jumpto
  (bind _canjump (CallFunction|CheckJump))
  (if _canjump
    (Variables|Default|SetLocation (+ (* (Math|Rotator|GetRotationXVector (Transformation|GetWorldRotation (Variables|Character|GetMesh))) (Math|Conversions|ToFloat(Integer) (Variables|/Game/BluePrints/CrossRoadAss.CrossRoadAss_C|GetMatrixSize (Variables|Default|GetGame)))) (Variables|Default|GetLocation)))
    (Variables|Default|SetIsJumping true)))

(fn GetCamera
  (Game|SpawnActorfromClass "/Script/Engine.CameraActor" (Math|Transform|MakeTransform (Math|Vector|MakeVector -3.5e+02 (.y (Variables|Default|GetLocation)) 3.5e+02) "0, 0, 0" "1,1,1") "Undefined" 0 0))

(fn Reset
  (Utilities|FlowControl|Sequence
    (:then_0
      (Transformation|SetActorLocation (Transformation|GetActorLocation (Class|GameModeBase|FindPlayerStart (Game|GetGameMode) (Game|GetPlayerController 0))) false false)
      (Variables|Default|SetonScreen false))
    (:then_1
      (Variables|Default|SetisDead false))
    (:then_2
      (Input|EnableInput 0))
    (:then_3
      (Variables|Default|SetIsJumping false)
      (Variables|Default|SetLocation (Transformation|GetActorLocation)))))

(fn PlacePlayer
  (bind _returnvalue (Transformation|GetActorLocation))
  (Transformation|SetActorLocation (Math|Vector|MakeVector (.x _returnvalue) (.y _returnvalue) 1.5e+02) false false))

(fn InitializePlayer
  (Utilities|FlowControl|Sequence
    (:then_0
      (Variables|Default|SetLocation (Transformation|GetWorldLocation (Variables|Character|GetMesh)))
      (Variables|Default|SetIsJumping false))
    (:then_1
      (Input|EnableInput (Game|GetPlayerController 0)))))

(fn OverlapControl
  (params (Actor :type Actor%20Object%20Reference))
  (bind _game (Variables|Default|GetGame))
  (if (Utilities|IsValid _game)
    (if (Variables|/Game/BluePrints/CrossRoadAss.CrossRoadAss_C|GetIsPlaying _game)
      _)))

(fn RoundtotheNearest50
  (params (Num :type Float%20%28single-precision%29))
  (bind _output_get (Variables|Default|SetRounded Num))
  (bind _output_get_2 (Variables|Default|SetRounded (Math|Conversions|ToFloat(Integer) (.ReturnValue (Math|Float|Division(WholeandRemainder) (+ _output_get 25.0) 5e+01)))))
  (return (* _output_get_2 5e+01)))