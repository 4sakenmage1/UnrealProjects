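; BP_Chicken is a chicken pawn moved by player input through the MoveForward and MoveRight mappings.
; Releasing either action adds movement input along X or Y, scaled by the matching axis value and MaxSpeed; the axis events themselves run no logic.
; Tick consumes the accumulated input vector and applies it as a delta-time-scaled local offset without sweep, so movement ignores collision.
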(event EventBeginPlay)

(event Collision|EventActorBeginOverlap
  (params (OtherActor :type Actor%20Object%20Reference)))

(event EventTick
  (params (DeltaSeconds :type Float%20%28single-precision%29))
  (bind _returnvalue (Class|Pawn|ConsumeMovementInputVector))
  (Transformation|AddActorLocalOffset (* _returnvalue DeltaSeconds) false false))

(event Input|ActionEvents|InputActionMoveForward
  (params (Key :type Key%20Structure))
  (:Released
    (Pawn|Input|AddMovementInput "10.000000, 0, 0" (* (stale Input|AxisEvents|InputAxisMoveForward AxisValue) (Variables|Default|GetMaxSpeed)) false)))

(event Input|ActionEvents|InputActionMoveRight
  (params (Key :type Key%20Structure))
  (:Released
    (Pawn|Input|AddMovementInput "0.000000,10.000000, 0" (* (stale Input|AxisEvents|InputAxisMoveRight AxisValue) (Variables|Default|GetMaxSpeed)) false)))

(event Input|ActionEvents|InputActionMoveForward
  (params (Key :type Key%20Structure)))

(event Input|AxisEvents|InputAxisMoveForward
  (params (AxisValue :type Float%20%28single-precision%29)))

(event Input|AxisEvents|InputAxisMoveRight
  (params (AxisValue :type Float%20%28single-precision%29)))

(fn ConstructionScript)