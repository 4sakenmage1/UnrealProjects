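; Side-view camera actor that follows the first player's pawn.
; Each Tick, FollowPlayer moves the Camera component to a fixed offset from the pawn, mostly along world Y and slightly raised.
; ShowPlayer then rotates the camera to look at the pawn's root component.
; A separate GetView function, not called here, makes this actor the player controller's view target.
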(event EventBeginPlay)

(event Collision|EventActorBeginOverlap
  (params (OtherActor :type Actor%20Object%20Reference)))

(event EventTick
  (params (DeltaSeconds :type Float%20%28single-precision%29))
  (CallFunction|FollowPlayer))

(fn ConstructionScript)

(fn FollowPlayer
  (bind _returnvalue (Game|Player|GetPlayerPawn 0))
  (bind _returnvalue_2 (Transformation|GetActorLocation _returnvalue))
  (if (Utilities|IsValid _returnvalue)
    (Transformation|SetWorldLocation (Variables|Default|GetCamera) (Math|Vector|MakeVector (.x _returnvalue_2) (+ (.y _returnvalue_2) 5e+01) (+ (.z _returnvalue_2) 1.0)) false false)
    (CallFunction|ShowPlayer)))

(fn ShowPlayer
  (Transformation|SetWorldRotation (Variables|Default|GetCamera) (Math|Conversions|RotationFromXVector (Math|Vector|GetUnitDirection(Vector) (Transformation|GetWorldLocation (Variables|Default|GetCamera)) (Transformation|GetWorldLocation (Variables|/Script/Engine.Actor|GetRootComponent (Game|Player|GetPlayerPawn 0))))) false false))

(fn GetView
  (Game|Player|SetViewTargetwithBlend (Game|GetPlayerController 0) self 0.0 "VTBlend_Linear" 0.0 false)
  (return false))