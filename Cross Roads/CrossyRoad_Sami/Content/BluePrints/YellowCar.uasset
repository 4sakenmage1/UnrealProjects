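; YellowCar is a moving car Actor that drives in a straight line and removes itself after about five seconds.
; Tick calls UseSpeed, a swept, frame-rate-independent offset along SpeedDirection scaled by Speed, then runs the Delay that leads to DestroyActor.
; SetRotation sets the car component's world rotation.
; Disconnected graph chains hold an unused looping version that teleports the car back to the Road's SpawnRight point.
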(event EventBeginPlay)

(event Collision|EventActorBeginOverlap
  (params (OtherActor :type Actor%20Object%20Reference)))

(event EventTick
  (params (DeltaSeconds :type Float%20%28single-precision%29))
  (CallFunction|UseSpeed DeltaSeconds)
  (Utilities|FlowControl|Delay 5.0)
  (Actor|DestroyActor))

(fn ConstructionScript)

(fn SetRotation
  (params (Rotation :type Rotator))
  (Transformation|SetWorldRotation (Variables|Default|GetYellowCar) Rotation false false))

(fn UseSpeed
  (params (DeltaSeconds :type Float%20%28single-precision%29))
  (Transformation|AddActorWorldOffset (* (* (Variables|Default|GetSpeedDirection) DeltaSeconds) (Variables|Default|GetSpeed)) true))