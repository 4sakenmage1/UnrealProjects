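; Crossy Road-style game manager that builds an endless map of grass, road, water and train track strips along X.
; BeginPlay spawns the opening strips, grass first and then random types, each placed by an incrementing index times tile size.
; Tick is meant to add strips as the player nears the edge, but IsPlaying is never set true here.
; Player lookup, death check, despawning and map clearing are empty or disconnected.
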(event EventBeginPlay
  (CallFunction|InitializeGame))

(event EventTick
  (params (DeltaSeconds :type Float%20%28single-precision%29))
  (CallFunction|CheckGame DeltaSeconds))

(event Input|ActionEvents|InputActionMoveForward
  (params (Key :type Key%20Structure))
  (:Released
    (Development|PrintString "Hello")))

(fn ConstructionScript)

(fn CreateGrass
  (Game|SpawnActorfromClass "/Game/Assets/Grass/Grass_BP.Grass_BP_C" (Math|Transform|MakeTransform (Math|Vector|MakeVector (* (Math|Conversions|ToFloat(Integer) (Variables|Default|GetNextSpawnX)) (Variables|Default|GetTileSize)) 0.0 0.0) "0, 0, 0" "2.000000,1,1") "Undefined" 0 0))

(fn CreateRoad
  (Game|SpawnActorfromClass "/Game/Assets/Road/Road_BP.Road_BP_C" (Math|Transform|MakeTransform (Math|Vector|MakeVector (* (Math|Conversions|ToFloat(Integer) (Variables|Default|GetNextSpawnX)) (Variables|Default|GetTileSize)) 0.0 0.0) "0, 0, 0" "2.000000,1,1") "Undefined" 0 0))

(fn CreateWater
  (Game|SpawnActorfromClass "/Game/Assets/Water/Water_BP.Water_BP_C" (Math|Transform|MakeTransform (Math|Vector|MakeVector (* (Math|Conversions|ToFloat(Integer) (Variables|Default|GetNextSpawnX)) (Variables|Default|GetTileSize)) 0.0 0.0) "0, 0, 0" "2.000000,1,1") "Undefined" 0 0))

(fn CreateTrainTracks
  (Game|SpawnActorfromClass "/Game/Assets/Tracks/TrainTracksBP.TrainTracksBP_C" (Math|Transform|MakeTransform (Math|Vector|MakeVector (* (Math|Conversions|ToFloat(Integer) (Variables|Default|GetNextSpawnX)) (Variables|Default|GetTileSize)) 0.0 0.0) "0, 0, 0" "2.000000,1,1") "Undefined" 0 0))

(fn CheckGame
  (params (deltaSeconds :type Float%20%28single-precision%29))
  (if (Variables|Default|GetIsPlaying)
    (Utilities|FlowControl|Sequence
      (:then_0
        (CallFunction|CheckPlayer))
      (:then_1
        (CallFunction|CheckSpawnTile))
      (:then_2
        (CallFunction|CheckDespawnTile)))))

(fn CheckPlayer)

(fn CheckSpawnTile
  (bind _player (Variables|Default|GetPlayer))
  (bind _returnvalue (Transformation|GetActorLocation _player))
  (bind _returnx (CallFunction|WorldtoMatrix (.x _returnvalue) (.y _returnvalue)))
  (if (>= _returnx (- (Variables|Default|GetNextSpawnX) (Variables|Default|GetNextTriggerDistance)))
    (CallFunction|SpawnNextTile)))

(fn CheckDespawnTile)

(fn InitializeGame
  (Utilities|FlowControl|Sequence
    (:then_0
      (Variables|Default|SetIsPlaying false))
    (:then_1
      (CallFunction|GetPlayer))
    (:then_2
      (CallFunction|InitializeCameraMain))
    (:then_3
      (CallFunction|NewMap)
      (for _index (range 0 50)
        (CallFunction|SpawnNextTile)))))

(fn GetPlayer)

(fn GetCamera
  (if (Variables|Default|GetisCamera)
    (Utilities|FlowControl|Sequence
      (:then_0
        (CallFunction|InitializeCameraMain))
      (:then_1
        (CallFunction|InitializeCameraSide))
      (:then_2
        (CallFunction|SetCamera)))))

(fn NewMap
  (Utilities|FlowControl|Sequence))

(fn MatrixtoWorld
  (params (xTiles :type Float%20%28single-precision%29) (yTiles :type Float%20%28single-precision%29))
  (bind _matrixsize (Variables|Default|GetMatrixSize))
  (return (* _matrixsize xTiles) (* _matrixsize yTiles)))

(fn WorldtoMatrix
  (params (X :type Float%20%28single-precision%29) (Y :type Float%20%28single-precision%29))
  (bind _matrixsize (Variables|Default|GetMatrixSize))
  (bind _returnvalue (Math|Conversions|ToFloat(Integer) _matrixsize))
  (return (Math|Float|Truncate (/ X _returnvalue)) (Math|Float|Truncate (/ Y _returnvalue))))

(fn SpawnNextTile
  (bind _nextspawnx (Variables|Default|GetNextSpawnX))
  (Math|Integer|IncrementInt _nextspawnx
    (:%20%20
      (if (< _nextspawnx 4)
        (CallFunction|CreateGrass :!label _label)
        (else
          (switch int (Math|Random|RandomInteger 4)
            (:0
              (goto _label))
            (:1
              (CallFunction|CreateRoad))
            (:2
              (CallFunction|CreateWater))
            (:3
              (CallFunction|CreateTrainTracks))))))))

(fn InitializeCameraMain
  (if (Variables|Default|GetisCamera)
    (Game|SpawnActorfromClass "/Game/BluePrints/Camera_Main.Camera_Main_C" (Math|Transform|MakeTransform "0, 0, 0" "0, 0, 0" "1,1,1") "Undefined" 0 0)))

(fn InitializeCameraSide
  (Utilities|FlowControl|Sequence
    (:then_0
      (if (Utilities|IsValid (Variables|Default|GetCamera_Side))
        (Actor|DestroyActor (Variables|Default|GetCamera_Side))))
    (:then_1
      (bind _returnvalue (Game|SpawnActorfromClass "/Game/BluePrints/Camera_Side.Camera_Side_C" (Math|Transform|MakeTransform "-500.000000,50.000000,150.000000" "0, 0, 0" "1,1,1") "Undefined" 0 0))
      (Variables|Default|SetCamera_Side _returnvalue))))

(fn SetCamera
  (if (Variables|Default|GetisCamera)
    (if (Variables|Default|GetIsCamera_Main)
      (Transformation|SetWorldLocation (Variables|/Game/BluePrints/Camera_Main.Camera_Main_C|GetDefaultSceneRoot (Variables|Default|GetCamera_Main)) (Transformation|GetWorldLocation (Variables|/Script/Engine.Character|GetMesh (Variables|Default|GetPlayer))) false false))))

(fn GetRound
  (Utilities|FlowControl|Sequence
    (:then_0
      (Variables|Default|SetIsPlaying false)
      (Default|Reset (Variables|Default|GetPlayer)))
    (:then_1
      (CallFunction|GetCamera))
    (:then_2
      (CallFunction|NewMap))))